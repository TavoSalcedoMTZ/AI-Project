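; BP_Arrow is an arrow projectile that an archer launches and that destroys itself on hitting a targetable actor.
; StartARROW stores the archer and sets forward velocity from charge value and the projectile's max speed.
; Tick fires an ArrowMovement dispatcher, to which launch binds a base movement event that damps velocity by frame time.
; Box overlap fetches the other actor's targetable component and, if valid, passes it the arrow type.
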(event OnComponentBeginOverlap(Box)
  (params (OverlappedComponent :type Primitive%20Component%20Object%20Reference) (OtherActor :type Actor%20Object%20Reference) (OtherComp :type Primitive%20Component%20Object%20Reference) (OtherBodyIndex :type Integer) (bFromSweep :type Boolean) (SweepResult :type Hit%20Result%20Structure%20%28by%20ref%29))
  (bind _comp (Class|BPIEnemy|GetTargeTableComponent(Message) OtherActor))
  (Utilities|IsValid _comp
    (:Is%20Valid
      (Class|BPITargeteableArrow|Hit(Message) _comp (Variables|Default|GetType%20Arrow))
      (Actor|DestroyActor))))

(event Custom|movementbase
  (bind _projectilemovement (Variables|Default|GetProjectileMovement))
  (Variables|/Script/Engine.MovementComponent|SetVelocity _projectilemovement (* (Variables|/Script/Engine.MovementComponent|GetVelocity _projectilemovement) (- 1.0 (* (Utilities|Time|GetWorldDeltaSeconds) 0.5)))))

(event Custom|StartARROW
  (params (archer :type BP%20Third%20Person%20Character%20Object%20Reference))
  (bind _projectilemovement (Variables|Default|GetProjectileMovement))
  (Variables|Default|SetArcher archer)
  (Variables|/Script/Engine.MovementComponent|SetVelocity _projectilemovement (* (Transformation|GetActorForwardVector) (* (Variables|Default|GetchargeValue) (Class|MovementComponent|GetMaxSpeed _projectilemovement))))
  (EventDispatchers|BindEventtoArrowMovement (delegate Custom|movementbase)))

(event EventTick
  (params (DeltaSeconds :type Float%20%28single-precision%29))
  (Default|CallArrowMovement))

(fn ConstructionScript)

(fn GetArrow
  (return self))