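; Enemy AI controller that runs the behavior tree defined on its BP_EnemyBase pawn and feeds it a player target.
; It caches the possessed pawn and starts that tree shortly after BeginPlay.
; Every tick it writes the nearer of players 0 and 1 to a blackboard key, falling back to whichever one is valid.
; The distance comparison sits behind a short Delay, throttling retargeting when both players exist.
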(event Custom|SetTarget
  (bind _returnvalue (Game|GetPlayerCharacter 0))
  (bind _returnvalue_2 (AI|GetBlackboard 0))
  (bind _returnvalue_3 (Game|GetPlayerCharacter 0))
  (bind _returnvalue_4 (Game|GetPlayerCharacter 1))
  (bind _returnvalue_5 (AI|GetBlackboard 0))
  (bind _returnvalue_6 (AI|GetBlackboard 0))
  (bind _returnvalue_7 (Game|GetPlayerCharacter 1))
  (bind _returnvalue_8 (Pawn|GetControlledPawn))
  (bind _returnvalue_9 (AI|GetBlackboard 0))
  (bind _returnvalue_10 (Game|GetPlayerCharacter 0))
  (bind _returnvalue_11 (Transformation|GetActorLocation _returnvalue_8))
  (Utilities|IsValid _returnvalue_10
    (:Is%20Valid
      (Utilities|IsValid _returnvalue_4
        (:Is%20Valid
          (Utilities|FlowControl|Delay 0.3)
          (if (< (Math|Vector|Distance(Vector) (Transformation|GetActorLocation _returnvalue_10) _returnvalue_11) (Math|Vector|Distance(Vector) _returnvalue_11 (Transformation|GetActorLocation _returnvalue_4)))
            (Utilities|IsValid _returnvalue_2
              (:Is%20Valid
                (Utilities|IsValid _returnvalue_3
                  (:Is%20Valid
                    (AI|Components|Blackboard|SetValueasObject _returnvalue_2 (Variables|Default|GetKey%20Name) _returnvalue_3)))))
            (else
              (Utilities|IsValid _returnvalue_5
                (:Is%20Valid
                  (Utilities|IsValid _returnvalue_5
                    (:Is%20Valid
                      (AI|Components|Blackboard|SetValueasObject _returnvalue_5 (Variables|Default|GetKey%20Name) (Game|GetPlayerCharacter 1)))))))))
        (:Is%20Not%20Valid
          (Utilities|IsValid _returnvalue
            (:Is%20Valid
              (Utilities|IsValid _returnvalue_9
                (:Is%20Valid
                  (AI|Components|Blackboard|SetValueasObject _returnvalue_9 (Variables|Default|GetKey%20Name) _returnvalue))))))))
    (:Is%20Not%20Valid
      (Utilities|IsValid _returnvalue_7
        (:Is%20Valid
          (Utilities|IsValid _returnvalue_6
            (:Is%20Valid
              (AI|Components|Blackboard|SetValueasObject _returnvalue_6 (Variables|Default|GetKey%20Name) _returnvalue_7))))))))

(event EventTick
  (params (DeltaSeconds :type Float%20%28single-precision%29))
  (CallFunction|SetTarget))

(event EventBeginPlay
  (Utilities|FlowControl|Delay 0.1)
  (bind _asbp_enemy_base (Utilities|Casting|CastToBP_EnemyBase (Variables|Default|GetSelf%20Pawn)))
  (AI|RunBehaviorTree (Variables|/Game/Armando/Enemies/BP_EnemyBase.BP_EnemyBase_C|GetBehaviorTreeAsset _asbp_enemy_base))
  (Utilities|FlowControl|Delay 0.05))

(event EventPossess
  (params (PossessedPawn :type Pawn%20Object%20Reference))
  (Variables|Default|SetSelf%20Pawn PossessedPawn))

(fn ConstructionScript)