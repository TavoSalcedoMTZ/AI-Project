(event Custom|TakeDamageCustom
  (params (DamageAmount :type Float%20%28double-precision%29))
  ;[0.15 0.15 0.15 0.5] Take Damage
  (if (not (Variables|Default|GetIsDead))
    (if (<= (Variables|Default|GetCurrentHealth) 0.0)
      (CallFunction|Die))))

(event Custom|Die
  ;[0.15 0.15 0.15 0.5] Die
  (Variables|Default|SetIsDead true)
  (Pawn|Components|CharacterMovement|DisableMovement (Variables|Character|GetCharacterMovement))
  (Collision|SetActorEnableCollision false)
  (Utilities|FlowControl|Delay 1.0)
  (Actor|DestroyActor))

(event EventBeginPlay
  ;[0.15 0.15 0.15 0.5] Initial Configuration
  (Variables|Default|SetCurrentHealth (Variables|Default|GetMaxHealth))
  (Variables|Default|SetTargetActor (Game|GetPlayerCharacter 0))
  (Variables|/Script/Engine.CharacterMovementComponent|SetMaxWalkSpeed (Variables|Character|GetCharacterMovement) (Variables|Default|GetMoveSpeed)))

(event EventTick
  (params (DeltaSeconds :type Float%20%28single-precision%29))
  ;[0.15 0.15 0.15 0.5] Persecution
)

(fn ConstructionScript)