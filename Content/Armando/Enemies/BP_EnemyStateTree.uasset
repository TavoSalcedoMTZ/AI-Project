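; Enemy Blueprint that provides a melee attack against a player actor passed into its PerformAttack event.
; When CanAttack is true, it calls AttackPlayer with fixed damage, prints a debug string and plays the melee montage on its mesh.
; CanAttack acts as a cooldown gate, cleared as the attack starts and restored only when the montage completes, with no handling for interruption.
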(event Custom|PerformAttack
  (params (NewParam :type Actor%20Object%20Reference))
  (if (Variables|Default|GetCanAttack)
    (CallFunction|AttackPlayer NewParam 1e+01)
    (Development|PrintString "Golpeando")
    (Variables|Default|SetCanAttack false)
    (Animation|Montage|PlayMontage (Variables|Character|GetMesh) "/Game/Armando/Enemies/Montage/AM_EnemyMeele.AM_EnemyMeele"
      (:OnCompleted
        (Variables|Default|SetCanAttack true)))))

(event EventBeginPlay
  (|CallParentFunction) ; This node is disabled and will not be called.\nDrag off pins to build functionality.
)

(event Collision|EventActorBeginOverlap
  (params (OtherActor :type Actor%20Object%20Reference)))

(event EventTick
  (params (DeltaSeconds :type Float%20%28single-precision%29))
  (|CallParentFunction DeltaSeconds) ; This node is disabled and will not be called.\nDrag off pins to build functionality.
)

(fn ConstructionScript
  (|CallParentFunction))