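; Game mode Blueprint that sets up local multiplayer by creating extra players when play begins.
; BeginPlay passes the SpawnPlayers count to SpawnPlayersFunc, which loops once per player.
; The first index only fetches the existing player controller; each later index calls CreatePlayer and, if valid, spawns a BP_ThirdPersonCharacter at the world origin.
; The function contains no explicit possession of the spawned characters.
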(event EventBeginPlay
  (CallFunction|SpawnPlayersFunc (Variables|Default|GetSpawnPlayers)))

(fn ConstructionScript)

(fn SpawnPlayersFunc
  (params (numOFSpawn :type Integer))
  (bind _index (Utilities|FlowControl|ForLoopwithBreak 0 (- numOFSpawn 1))
    (:LoopBody
      (if (== _index 0)
        (Game|GetPlayerController 0)
        (else
          (bind _returnvalue (Class|GameplayStatics|CreatePlayer _index))
          (Utilities|IsValid _returnvalue
            (:Is%20Valid
              (Game|SpawnActorfromClass "/Game/ThirdPerson/Blueprints/BP_ThirdPersonCharacter.BP_ThirdPersonCharacter_C" (Math|Transform|MakeTransform "0, 0, 0") "Undefined" "MultiplyWithRoot" 0 0))))))))